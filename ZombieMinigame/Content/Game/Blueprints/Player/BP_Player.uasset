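; Player character for a cursor-aimed shooter, with a socket-attached gun, ammo and health.
; Tick applies Enhanced Input movement relative to control yaw and smoothly turns the actor toward the point under the cursor.
; Firing spends ammo, and clamped ammo and health changes are broadcast through change notifications.
; A DoOnce with delayed reset gives a damage cooldown, and death ragdolls the mesh with an impulse along the damage causer's forward vector.
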(event Input|EnhancedActionEvents|EnhancedInputActionIA_FireWeapon
  (params (ActionValue :type Boolean) (ElapsedSeconds :type Float%20%28double-precision%29) (TriggeredSeconds :type Float%20%28double-precision%29) (InputAction :type Input%20Action%20Object%20Reference :default "/Game/Game/Input/Actions/IA_FireWeapon.IA_FireWeapon"))
  (:Started
    (bind _bcanfire (Weapon|CanFire))
    (if _bcanfire
      (Weapon|SpendAmmo 1)
      (Default|Fire (Variables|Weapon|GetGun%20Ref)))))

(event EventTick
  (params (DeltaSeconds :type Float%20%28single-precision%29))
  (Input|HandleMovement DeltaSeconds)
  (Input|HandleRotation DeltaSeconds))

(event EventBeginPlay
  ;[0.05098 0.05098 0.05098] Add Mapping Context And Initialize Variables
  (Utilities|FlowControl|Sequence
    (:then_0
      (Initialize|InitializeMesh))
    (:then_1
      (Initialize|InitializeVariables))
    (:then_2
      (Initialize|AddMappingContext))))

(event Game|Damage|EventAnyDamage
  (params (Damage :type Float%20%28single-precision%29) (DamageType :type Damage%20Type%20Object%20Reference) (InstigatedBy :type Controller%20Object%20Reference) (DamageCauser :type Actor%20Object%20Reference))
  (bind _returnvalue (Transformation|GetActorForwardVector DamageCauser))
  (bind _mesh (Variables|Character|GetMesh))
  (bind _impulseforce (Variables|Others|GetImpulseForce))
  (bind _returnvalue_2 (* _returnvalue _impulseforce))
  (Utilities|FlowControl|DoOnce false :!label _label
    (:Completed
      (Health|RemoveHealt 1)
      (if (<= (Variables|Health|GetHealth) 0)
        (Collision|SetCollisionProfileName _mesh "Ragdoll" false :!class /Script/Engine.PrimitiveComponent)
        (Physics|SetSimulatePhysics _mesh true)
        (Physics|AddImpulse _mesh (Math|Vector|MakeVector (.x _returnvalue_2) (.y _returnvalue_2) 0.0) "None" true)
        (Collision|SetCollisionEnabled (Variables|Collision|GetCapsuleComponent) "NoCollision")
        (else
          (Utilities|FlowControl|Delay (Variables|Health|GetDamage%20Cooldown))
          (goto _label Reset))))))

(fn ConstructionScript)

(fn HandleMovement
  (params (Delta%20Seconds :type Float%20%28double-precision%29))
  (bind _returnvalue (Pawn|GetControlRotation :!class /Script/Engine.Pawn))
  (Utilities|FlowControl|Sequence
    (:then_0
      (Pawn|Input|AddMovementInput (Math|Vector|GetRightVector (Math|Rotator|MakeRotator (.roll _returnvalue) 0.0 (.yaw _returnvalue))) (.x (Input|EnhancedActionValues|GetIA_Move)) false))
    (:then_1
      (Pawn|Input|AddMovementInput (Math|Vector|GetForwardVector (Math|Rotator|MakeRotator 0.0 0.0 (.yaw (Pawn|GetControlRotation :!class /Script/Engine.Pawn)))) (.y (Input|EnhancedActionValues|GetIA_Move)) false))))

(fn HandleRotation
  (params (Delta%20Seconds :type Float%20%28double-precision%29))
  (bind _returnvalue (Transformation|GetActorRotation))
  (Transformation|SetActorRotation (Math|Rotator|MakeRotator (.roll _returnvalue) (.pitch _returnvalue) (.yaw (Class|KismetMathLibrary|RInterptoConstant (Transformation|GetActorRotation) (Math|Rotator|FindLookatRotation (+ "" "") (- (.ImpactPoint (Collision|BreakHitResult (.HitResult (Game|Player|GetHitResultUnderCursorbyChannel (Variables|Others|GetPC%20Gameplay%20REF) "TraceTypeQuery1" true)))) (Transformation|GetActorLocation))) Delta%20Seconds (LocalVariables|GetInterp%20Speed))))))

(fn InitializeVariables
  (bind _aspc_gameplay (Utilities|Casting|CastToPC_Gameplay (Pawn|GetController)))
  (Variables|Others|SetPC%20Gameplay%20REF _aspc_gameplay))

(fn AddMappingContext
  (bind _pc_gameplay_ref (Variables|Others|GetPC%20Gameplay%20REF)
    (:then
      (Utilities|IsValid _pc_gameplay_ref
        (:Is%20Valid
          (Input|AddMappingContext (PlayerController|LocalPlayerSubsystems|GetEnhancedInputLocalPlayerSubsystem _pc_gameplay_ref) "/Game/Game/Input/IMC_Zombie.IMC_Zombie" 0 "(bIgnoreAllPressedKeysUntilRelease=True,bForceImmediately=False,bNotifyUserSettings=False)"))))
    (:else)))

(fn InitializeMesh
  (bind _returnvalue (Game|SpawnActorfromClass "/Game/Game/Blueprints/Gun/BP_Gun.BP_Gun_C" (Transformation|GetActorTransform) "Undefined" "MultiplyWithRoot" 0 0))
  (bind _output_get (Variables|Weapon|SetGun%20Ref _returnvalue))
  (Transformation|AttachComponentToComponent _output_get (Variables|Character|GetMesh) "GunSocket" "SnapToTarget" "SnapToTarget" "SnapToTarget" true))

(fn AddAmmo
  (params (Amount :type Integer))
  (Variables|Weapon|SetAmmo (Math|Integer|Clamp(Integer) (+ Amount (Variables|Weapon|GetAmmo)) 0 (Variables|Weapon|GetMax%20Ammo)))
  (CallFunction|CallonAmmoChangedFunction))

(fn SpendAmmo
  (params (Amount :type Integer))
  (Variables|Weapon|SetAmmo (Math|Integer|Clamp(Integer) (- (Variables|Weapon|GetAmmo) Amount) 0 (Variables|Weapon|GetMax%20Ammo)))
  (CallFunction|CallonAmmoChangedFunction))

(fn CanFire
  (return (> (Variables|Weapon|GetAmmo) 0)))

(fn CallonAmmoChangedFunction
  (Default|CallOnAmmoChanged (Variables|Weapon|GetAmmo) (Variables|Weapon|GetMax%20Ammo)))

(fn CallonHealthChangedFunction
  (params (bPlayBloodEffect :type Boolean))
  (Default|CallOnHealthChanged (Variables|Health|GetHealth) (Variables|Health|GetMax%20Health) bPlayBloodEffect))

(fn AddHealth
  (params (Amount :type Integer))
  (Variables|Health|SetHealth (Math|Integer|Clamp(Integer) (+ Amount (Variables|Health|GetHealth)) 0 (Variables|Health|GetMax%20Health)))
  (CallFunction|CallonHealthChangedFunction false))

(fn RemoveHealt
  (params (Amount :type Integer))
  (Variables|Health|SetHealth (Math|Integer|Clamp(Integer) (- (Variables|Health|GetHealth) Amount) 0 (Variables|Health|GetMax%20Health)))
  (CallFunction|CallonHealthChangedFunction true))