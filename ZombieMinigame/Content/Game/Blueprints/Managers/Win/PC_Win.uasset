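; Player controller for the win screen that creates the WBP_Win widget on BeginPlay and adds it to the viewport.
; It also carries top-down movement helpers: MoveTo paths to a location with a cursor Niagara effect, and Follow steers the pawn toward a point.
; Two trace functions return the visibility hit under the cursor or first finger, but no graph here calls any of these helpers.
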(event EventBeginPlay
  (bind _returnvalue (UserInterface|CreateWidget "/Game/Game/Widgets/Win/WBP_Win.WBP_Win_C"))
  (bind _output_get (Variables|Default|SetWin%20REF _returnvalue))
  (UserInterface|Viewport|AddtoViewport _output_get 0))

(fn ConstructionScript)

(fn Moveto
  (params (Location :type Vector))
  (AI|Navigation|SimpleMovetoLocation self Location)
  (Niagara|SpawnSystematLocation (Variables|Input|GetFXCursor) Location))

(fn Follow
  (params (Location :type Vector))
  (bind _returnvalue (Pawn|GetControlledPawn))
  (Pawn|Input|AddMovementInput _returnvalue (Math|Vector|GetUnitDirection(Vector) (Transformation|GetActorLocation _returnvalue) Location) 1.0 false))

(fn GetLocationUnderCursor
  (bind _hitresult (Game|Player|GetHitResultUnderCursorbyChannel "TraceTypeQuery1" true))
  (bind (_bblockinghit _binitialoverlap _time _distance _location) (Collision|BreakHitResult _hitresult))
  (return _bblockinghit _location))

(fn GetLocationUnderFinger
  (bind _hitresult (Class|PlayerController|GetHitResultUnderFingerbyChannel "Touch1" "TraceTypeQuery1" false))
  (bind (_bblockinghit _binitialoverlap _time _distance _location) (Collision|BreakHitResult _hitresult))
  (return _bblockinghit _location))