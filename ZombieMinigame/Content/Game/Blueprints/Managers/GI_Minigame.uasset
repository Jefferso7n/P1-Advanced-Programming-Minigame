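; Game instance for a minigame that persists the high score and carries the last match score for the session.
; On Init it loads the BP_SaveGame from the "Default" slot, or creates one in memory if that fails, and caches the reference.
; SaveHighscore overwrites the stored value without comparison and writes the slot, while the last match score stays only on the instance.
; Both getters reload the save before returning the high score.
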(event EventInit
  (CallFunction|CreateorUpdateSaveGame))

(fn SaveHighscore
  (params (NewHighScore :type Integer))
  (bind _bp_save_game_ref (Variables|Default|GetBP%20Save%20Game%20REF))
  (Variables|/Game/Game/Blueprints/SaveGame/BP_SaveGame.BP_SaveGame_C|SetHighScore _bp_save_game_ref NewHighScore)
  (SaveGame|SaveGametoSlot _bp_save_game_ref "Default"))

(fn CreateorUpdateSaveGame
  (bind _returnvalue (SaveGame|LoadGamefromSlot "Default"))
  (bind _asbp_save_game (Utilities|Casting|CastToBP_SaveGame _returnvalue)
    (:then
      (bind _output_get (Variables|Default|SetBP%20Save%20Game%20REF _asbp_save_game))
      (return _output_get))
    (:CastFailed
      (bind _returnvalue_2 (SaveGame|CreateSaveGameObject "/Game/Game/Blueprints/SaveGame/BP_SaveGame.BP_SaveGame_C"))
      (bind _output_get_2 (Variables|Default|SetBP%20Save%20Game%20REF _returnvalue_2))
      (return _output_get_2))))

(fn GetHighscore
  (bind _bp_save_game (CallFunction|CreateorUpdateSaveGame))
  (return (Variables|/Game/Game/Blueprints/SaveGame/BP_SaveGame.BP_SaveGame_C|GetHighScore _bp_save_game)))

(fn SaveLastMatch
  (params (Last%20Match%20Score :type Integer))
  (Variables|Default|SetLast%20Match%20Score Last%20Match%20Score))

(fn GetLastMatchScores
  (bind _bp_save_game (CallFunction|CreateorUpdateSaveGame))
  (return (Variables|Default|GetLast%20Match%20Score) (Variables|/Game/Game/Blueprints/SaveGame/BP_SaveGame.BP_SaveGame_C|GetHighScore _bp_save_game)))