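; Gameplay player controller that creates the HUD and relays the player's ammo and health changes to it.
; On BeginPlay it caches the BP_Player pawn, adds WBP_HUD, binds both change delegates and triggers an initial refresh of each.
; It also holds top-down movement helpers for cursor and touch traces, move-to with cursor FX and follow input, none of which are called in this file.
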(event Custom|OnAmmoChanged_Event
  (params (Current%20Ammo :type Integer) (Max%20Ammo :type Integer))
  ;[0 0 0] Bind Ammo
  (Default|OnAmmoChanged (Variables|Default|GetHUD%20Ref) Current%20Ammo Max%20Ammo))

(event Custom|OnHealthChanged_Event
  (params (Current%20Health :type Integer) (Max%20Health :type Integer) (bPlayBloodEffect :type Boolean))
  ;[0 0 0] Bind Health
  (Default|OnHealthChanged (Variables|Default|GetHUD%20Ref) Current%20Health Max%20Health bPlayBloodEffect))

(event EventBeginPlay
  (Utilities|FlowControl|Sequence
    (:then_0
      (bind _asbp_player (Utilities|Casting|CastToBP_Player (Pawn|GetControlledPawn)))
      (Variables|Default|SetPlayer%20Ref _asbp_player))
    (:then_1
      (bind _returnvalue (UserInterface|CreateWidget "/Game/Game/Widgets/WBP_HUD.WBP_HUD_C"))
      (bind _output_get (Variables|Default|SetHUD%20Ref _returnvalue))
      (UserInterface|Viewport|AddtoViewport _output_get 0))
    (:then_2
      ;[0 0 0] Bind Ammo
      (EventDispatchers|AssignOnAmmoChanged (Variables|Default|GetPlayer%20Ref) (delegate Custom|OnAmmoChanged_Event))
      (Default|CallonAmmoChangedFunction (Variables|Default|GetPlayer%20Ref)))
    (:then_3
      ;[0 0 0] Bind Health
      (EventDispatchers|AssignOnHealthChanged (Variables|Default|GetPlayer%20Ref) (delegate Custom|OnHealthChanged_Event))
      (Default|CallonHealthChangedFunction (Variables|Default|GetPlayer%20Ref) false))))

(fn ConstructionScript)

(fn Moveto
  (params (Location :type Vector))
  (AI|Navigation|SimpleMovetoLocation self Location)
  (Niagara|SpawnSystematLocation (Variables|Input|GetFXCursor) Location))

(fn Follow
  (params (Location :type Vector))
  (bind _returnvalue (Pawn|GetControlledPawn))
  (Pawn|Input|AddMovementInput _returnvalue (Math|Vector|GetUnitDirection(Vector) (Transformation|GetActorLocation _returnvalue) Location) 1.0 false))

(fn GetLocationUnderCursor
  (bind _hitresult (Game|Player|GetHitResultUnderCursorbyChannel "TraceTypeQuery1" true))
  (bind (_bblockinghit _binitialoverlap _time _distance _location) (Collision|BreakHitResult _hitresult))
  (return _bblockinghit _location))

(fn GetLocationUnderFinger
  (bind _hitresult (Class|PlayerController|GetHitResultUnderFingerbyChannel "Touch1" "TraceTypeQuery1" false))
  (bind (_bblockinghit _binitialoverlap _time _distance _location) (Collision|BreakHitResult _hitresult))
  (return _bblockinghit _location))