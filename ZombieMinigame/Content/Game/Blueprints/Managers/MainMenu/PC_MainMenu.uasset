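; Player controller for the main menu that shows the menu widget and the saved high score.
; On BeginPlay it creates WBP_MainMenu, then loads the Default save slot and passes its BP_SaveGame high score to the widget.
; It also defines click-to-move, follow and cursor/touch trace helpers, none of which are called in its own graphs.
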(event EventBeginPlay
  (Utilities|FlowControl|Sequence
    (:then_0
      (bind _returnvalue (UserInterface|CreateWidget "/Game/Game/Widgets/MainMenu/WBP_MainMenu.WBP_MainMenu_C"))
      (bind _output_get (Variables|Default|SetMain%20Menu%20Ref _returnvalue))
      (UserInterface|Viewport|AddtoViewport _output_get 0))
    (:then_1
      (bind _returnvalue_2 (SaveGame|LoadGamefromSlot "Default"))
      (bind _asbp_save_game (Utilities|Casting|CastToBP_SaveGame _returnvalue_2))
      (Default|UpdateScoreText (Variables|Default|GetMain%20Menu%20Ref) (Variables|/Game/Game/Blueprints/SaveGame/BP_SaveGame.BP_SaveGame_C|GetHighScore _asbp_save_game)))))

(fn ConstructionScript)

(fn Moveto
  (params (Location :type Vector))
  (AI|Navigation|SimpleMovetoLocation self Location)
  (Niagara|SpawnSystematLocation (Variables|Input|GetFXCursor) Location))

(fn Follow
  (params (Location :type Vector))
  (bind _returnvalue (Pawn|GetControlledPawn))
  (Pawn|Input|AddMovementInput _returnvalue (Math|Vector|GetUnitDirection(Vector) (Transformation|GetActorLocation _returnvalue) Location) 1.0 false))

(fn GetLocationUnderCursor
  (bind _hitresult (Game|Player|GetHitResultUnderCursorbyChannel "TraceTypeQuery1" true))
  (bind (_bblockinghit _binitialoverlap _time _distance _location) (Collision|BreakHitResult _hitresult))
  (return _bblockinghit _location))

(fn GetLocationUnderFinger
  (bind _hitresult (Class|PlayerController|GetHitResultUnderFingerbyChannel "Touch1" "TraceTypeQuery1" false))
  (bind (_bblockinghit _binitialoverlap _time _distance _location) (Collision|BreakHitResult _hitresult))
  (return _bblockinghit _location))