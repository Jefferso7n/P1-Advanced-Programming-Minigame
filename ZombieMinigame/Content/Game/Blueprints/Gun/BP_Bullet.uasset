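; BP_Bullet is a reusable gun projectile that damages what it hits.
; It extends the parent's in-use toggle, launching along its forward vector at bullet speed when activated and zeroing velocity when deactivated.
; On sphere overlap with any actor not tagged "ignore", it applies bullet damage with itself as causer, then marks itself out of use instead of being destroyed.
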(event OnComponentBeginOverlap(Sphere)
  (params (OverlappedComponent :type Primitive%20Component%20Object%20Reference) (OtherActor :type Actor%20Object%20Reference) (OtherComp :type Primitive%20Component%20Object%20Reference) (OtherBodyIndex :type Integer) (bFromSweep :type Boolean) (SweepResult :type Hit%20Result%20Structure%20%28by%20ref%29))
  (if (not (Actor|ActorHasTag OtherActor "ignore"))
    (Game|Damage|ApplyDamage OtherActor (Math|Conversions|ToFloat(Integer) (Variables|Default|GetBullet%20Damage)) 0 self)
    (CallFunction|SetinUse false)))

(event EventSetinUse
  (params (InUse :type Boolean))
  (|CallParentFunction InUse)
  (if InUse
    (Variables|/Script/Engine.MovementComponent|SetVelocity (Variables|Default|GetProjectileMovement) (* (Transformation|GetActorForwardVector) (Variables|Default|GetBullet%20Speed)))
    (else
      (Variables|/Script/Engine.MovementComponent|SetVelocity (Variables|Default|GetProjectileMovement) "0, 0, 0"))))

(fn ConstructionScript)