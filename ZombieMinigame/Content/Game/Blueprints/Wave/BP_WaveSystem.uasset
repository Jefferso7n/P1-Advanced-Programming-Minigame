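; Wave manager that runs endless zombie waves, each larger than the last, starting on BeginPlay.
; Each wave shows a countdown widget, then pulls zombies from a character pool at random spawn points with a magic-circle effect.
; It also spawns a first aid kit and an ammo pickup scaled to the enemy count.
; RemoveZombie triggers a fixed sphere-overlap health check, advancing the wave when no living zombie remains inside.
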(event Custom|Start%20Wave
  (bind _returnvalue (UserInterface|CreateWidget "/Game/Game/Widgets/HUD/WBP_WaveTimer.WBP_WaveTimer_C" 0 (Variables|Default|GetWave%20Transition%20Time)))
  (bind _output_get (Variables|Default|SetWave%20Timer%20REF _returnvalue))
  (UserInterface|Viewport|AddtoViewport _output_get 0)
  (Utilities|FlowControl|Delay (Math|Conversions|ToFloat(Integer) (Variables|Default|GetWave%20Transition%20Time)))
  (for _index (range 0 (+ (* (Variables|Default|GetCurrent%20Wave) 2) 3))
    (bind _output_get_2 (Variables|Default|SetSpawn%20Point%20Transform (CallFunction|GetRandomZombieSpawnPointTransform)))
    (bind _pooledactor (Default|SpawnfromPool (Variables|Default|GetAC_CharacterPool) _output_get_2))
    (Utilities|Array|Add (Variables|Default|GetEnemies%20Alive) _pooledactor)
    (bind _asbp_zombie (Utilities|Casting|CastToBP_Zombie _pooledactor))
    (Variables|/Game/Game/Blueprints/Zombies/BP_Zombie.BP_Zombie_C|SetWave%20System%20REF _asbp_zombie self)
    (Niagara|SpawnSystematLocation "/Game/_Game/Vfx/Fx/Systems/NS_MagicCircle.NS_MagicCircle" (.Location (Math|Transform|BreakTransform _output_get_2))))
  (Utilities|FlowControl|Sequence
    (:then_0
      (Game|SpawnActorfromClass "/Game/Game/Blueprints/PickUps/BP_PickUp_Ammo.BP_PickUp_Ammo_C" (CallFunction|GetRandomAmmoSpawnPointTransform) "AdjustIfPossibleButAlwaysSpawn" "MultiplyWithRoot" 0 (+ (* (Utilities|Array|Length (Variables|Default|GetEnemies%20Alive)) 3) 25) 0))
    (:then_1
      (Game|SpawnActorfromClass "/Game/Game/Blueprints/PickUps/BP_PickuUp_FirstAidKit.BP_PickuUp_FirstAidKit_C" (CallFunction|GetRandomFirstAidKitSpawnPointTransform) "AdjustIfPossibleButAlwaysSpawn" "MultiplyWithRoot" 0 0))))

(event Custom|Check%20Wave
  (bind _outactors (Collision|SphereOverlapActors "2380.000000,2250.000000,0.000000" 3.5e+03 (Utilities|Array|MakeArray "ObjectTypeQuery3") "/Game/Game/Blueprints/Zombies/BP_Zombie.BP_Zombie_C"))
  (Variables|Default|SetCanMoveToNextWave true)
  (for _array_element _outactors
    (bind _asbp_zombie (Utilities|Casting|CastToBP_Zombie _array_element))
    (if (> (Variables|/Game/Game/Blueprints/Zombies/BP_Zombie.BP_Zombie_C|GetHealth _asbp_zombie) 0.0)
      (Variables|Default|SetCanMoveToNextWave false)))
  (if (Variables|Default|GetCanMoveToNextWave)
    (Variables|Default|SetCurrent%20Wave (+ (Variables|Default|GetCurrent%20Wave) 1))
    (CallFunction|StartWave)))

(event EventBeginPlay
  (CallFunction|StartWave))

(fn ConstructionScript)

(fn GetRandomZombieSpawnPointTransform
  (return (Transformation|GetWorldTransform (Variables|/Game/Game/Blueprints/Wave/BP_ZombieSpawnPoint.BP_ZombieSpawnPoint_C|GetDefaultSceneRoot (.OutItem (Utilities|Array|Random (Variables|Spawn|GetZombie%20Spawn%20Points)))))))

(fn GetRandomAmmoSpawnPointTransform
  (return (Transformation|GetWorldTransform (Variables|/Script/Engine.Actor|GetRootComponent (.OutItem (Utilities|Array|Random (Variables|Spawn|GetAmmo%20Spawn%20Points)))))))

(fn RemoveZombie
  (params (Item :type BP%20Pooled%20Character%20Object%20Reference%20%28by%20ref%29))
  (Utilities|Array|RemoveItem (Variables|Default|GetEnemies%20Alive) Item)
  (CallFunction|CheckWave))

(fn GetRandomFirstAidKitSpawnPointTransform
  (return (Transformation|GetWorldTransform (Variables|/Game/Game/Blueprints/Wave/BP_FirstAidKitSpawnPoint.BP_FirstAidKitSpawnPoint_C|GetDefaultSceneRoot (.OutItem (Utilities|Array|Random (Variables|Spawn|GetFirst%20Aid%20Kit%20Spawn%20Points)))))))