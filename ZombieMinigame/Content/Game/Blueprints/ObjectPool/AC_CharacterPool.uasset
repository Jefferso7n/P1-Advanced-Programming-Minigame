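; Actor component that pools characters, treated as BP_Zombie, so they can be reused when spawning.
; On BeginPlay it pre-spawns PoolSize actors of PooledCharacterClass marked not in use and caches the BP_WaveSystem reference.
; SpawnFromPool takes the first free zombie, moves it to the requested transform and marks it in use.
; When none is free, the pool grows by spawning another and prints a debug message.
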(event Custom|InitializePool
  (for _index (range 0 (Variables|Default|GetPoolSize))
    (bind _returnvalue (Game|SpawnActorfromClass (Variables|Default|GetPooledCharacterClass) (Math|Transform|MakeTransform "0.000000,0.000000,-90.000000" "0.000000,-90.000000,0.000000" "1.000000,1.000000,1.000000") "AdjustIfPossibleButAlwaysSpawn" "MultiplyWithRoot" 0 0.0 0))
    (Utilities|Array|AddUnique (Variables|Default|GetObjectPool) _returnvalue)
    (Default|SetinUse _returnvalue false)))

(event EventBeginPlay
  (CallFunction|InitializePool)
  (bind _outactors (Actor|GetAllActorsOfClass "/Game/Game/Blueprints/Wave/BP_WaveSystem.BP_WaveSystem_C"))
  (Variables|Default|SetWave%20System%20REF (Utilities|Array|Get(acopy) _outactors)))

(fn FindFirstAvailableCharacter
  (for _array_element (Variables|Default|GetObjectPool)
    (bind _asbp_zombie (Utilities|Casting|CastToBP_Zombie _array_element))
    (if (not (Variables|/Game/Game/Blueprints/ObjectPool/BP_PooledCharacter.BP_PooledCharacter_C|GetbInUse _asbp_zombie))
      (return _array_element)))
  ;[0 0 0] Expand Pool
  (bind _returnvalue (Game|SpawnActorfromClass (Variables|Default|GetPooledCharacterClass) (Math|Transform|MakeTransform "0.000000,0.000000,-90.000000" "0.000000,-90.000000,0.000000" "1.000000,1.000000,1.000000") "AdjustIfPossibleButAlwaysSpawn" "MultiplyWithRoot" 0 0.0 0))
  (Utilities|Array|AddUnique (Variables|Default|GetObjectPool) _returnvalue)
  (Default|SetinUse _returnvalue false)
  (Development|PrintString "EXPAND POOL" true true "(R=1.000000,G=0.070010,B=0.000000,A=1.000000)" 1.0)
  (return _returnvalue))

(fn SpawnfromPool
  (params (SpawnTransform :type Transform))
  (bind _pooledcharacter (CallFunction|FindFirstAvailableCharacter))
  (Utilities|IsValid _pooledcharacter
    (:Is%20Valid
      (Transformation|SetActorTransform _pooledcharacter SpawnTransform)
      (Default|SetinUse _pooledcharacter true)
      (return _pooledcharacter))
    (:Is%20Not%20Valid
      (Development|PrintString "Failed To Spawn Character From Pool"))))