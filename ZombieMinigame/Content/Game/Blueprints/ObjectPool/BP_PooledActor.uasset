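; BP_PooledActor is a base actor for an object pool, toggled between active and inactive instead of being spawned and destroyed.
; SetInUse flips collision, ticking and visibility, and the actor starts inactive on BeginPlay.
; Activation starts a time-to-live timer that calls ReturnToPool to deactivate it, and every state change clears any pending timer first.
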(event Custom|SetInUse
  (params (InUse :type Boolean))
  (bind _output_get (Variables|Default|SetbInUse InUse))
  (Collision|SetActorEnableCollision _output_get)
  (Actor|Tick|SetActorTickEnabled _output_get)
  (Rendering|SetActorHiddenInGame (not _output_get))
  (Utilities|Time|ClearandInvalidateTimerbyHandle (Variables|Default|GetTime%20To%20Live%20Timer))
  (if InUse
    (bind _returnvalue (Utilities|Time|SetTimerbyEvent (delegate Custom|ReturnToPool) (Variables|Default|GetTimeToLive)))
    (Variables|Default|SetTime%20To%20Live%20Timer _returnvalue)))

(event Custom|ReturnToPool
  (CallFunction|SetinUse false))

(event EventBeginPlay
  (CallFunction|SetinUse false))

(fn ConstructionScript)