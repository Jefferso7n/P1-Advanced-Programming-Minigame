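; BP_Zombie is a wave enemy that chases the player, reissuing AIMoveTo every Tick.
; Capsule overlap with the player toggles IsAttacking while it is alive.
; Damage spawns a splash effect; at zero health it ragdolls with an impulse from the damage causer, leaves the wave system, awards score and is destroyed after a delay.
; The older roaming and PawnSensing chase logic remains but is disconnected.
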(event OnSeePawn(PawnSensing)
  (params (Pawn :type Pawn%20Object%20Reference))
  ;[1 0 0] Movimentação antiga de roaming / Seguir player
)

(event OnComponentBeginOverlap(Capsule)
  (params (OverlappedComponent :type Primitive%20Component%20Object%20Reference) (OtherActor :type Actor%20Object%20Reference) (OtherComp :type Primitive%20Component%20Object%20Reference) (OtherBodyIndex :type Integer) (bFromSweep :type Boolean) (SweepResult :type Hit%20Result%20Structure%20%28by%20ref%29))
  (if (== OtherActor (Variables|Default|GetBP%20Player%20REF))
    (if (> (Variables|Default|GetHealth) 0.0)
      (Variables|Default|SetbIsAttacking true))))

(event OnComponentEndOverlap(Capsule)
  (params (OverlappedComponent :type Primitive%20Component%20Object%20Reference) (OtherActor :type Actor%20Object%20Reference) (OtherComp :type Primitive%20Component%20Object%20Reference) (OtherBodyIndex :type Integer))
  (if (== OtherActor (Variables|Default|GetBP%20Player%20REF))
    (if (> (Variables|Default|GetHealth) 0.0)
      (Variables|Default|SetbIsAttacking false))))

(event Custom|MoveAroundMap
  ;[1 0 0] Movimentação antiga de roaming / Seguir player
  (Variables|Default|SetbIsRunning false :!label _label)
  (bind _randomlocation (Class|NavigationSystemV1|GetRandomLocationinNavigableRadius (Transformation|GetActorLocation) (Variables|Default|GetRadius) 0 0))
  (AI|AIMoveTo self _randomlocation 0 5.0 false
    (:then
      (Utilities|FlowControl|Delay (Variables|Default|GetDuration))
      (if (not (Variables|Default|GetbCanSeePlayer))
        (goto _label)))))

(event Custom|Move%20To%20Player
  (AI|AIMoveTo self "0, 0, 0" (Variables|Default|GetBP%20Player%20REF) 5.0 false))

(event EventBeginPlay
  (bind _asbp_player (Utilities|Casting|CastToBP_Player (Game|Player|GetPlayerPawn 0)))
  (Variables|Default|SetBP%20Player%20REF _asbp_player))

(event EventTick
  (params (DeltaSeconds :type Float%20%28single-precision%29))
  (CallFunction|MovetoPlayer))

(event Game|Damage|EventAnyDamage
  (params (Damage :type Float%20%28single-precision%29) (DamageType :type Damage%20Type%20Object%20Reference) (InstigatedBy :type Controller%20Object%20Reference) (DamageCauser :type Actor%20Object%20Reference))
  (bind _returnvalue (Transformation|GetActorForwardVector DamageCauser))
  (bind _mesh (Variables|Character|GetMesh))
  (bind _impulseforce (Variables|Default|GetImpulseForce))
  (bind _returnvalue_2 (* _returnvalue _impulseforce))
  (bind _output_get (Variables|Default|SetHealth (- (Variables|Default|GetHealth) Damage)))
  (Niagara|SpawnSystemAttached (select (<= _output_get 0.0) "/Game/Blood_VFX_Pack/Particles/Systems/P_Splash_Burst_SkMesh.P_Splash_Burst_SkMesh" "/Game/Blood_VFX_Pack/Particles/Systems/P_BigSplash.P_BigSplash") (Variables|Character|GetMesh) "None" (Transformation|GetActorLocation) "0, 0, 0" "KeepWorldPosition" true)
  (if (<= _output_get 0.0)
    (Utilities|FlowControl|Sequence
      (:then_0
        (Collision|SetCollisionProfileName _mesh "Ragdoll" false :!class /Script/Engine.PrimitiveComponent)
        (Physics|SetSimulatePhysics _mesh true)
        (Physics|AddImpulse _mesh (Math|Vector|MakeVector (.x _returnvalue_2) (.y _returnvalue_2) 0.0) "None" true)
        (Collision|SetCollisionEnabled (Variables|Collision|GetCapsuleComponent) "NoCollision")
        (Default|RemoveZombie (Variables|Default|GetWave%20System%20REF) (Variables|Default|GetZombieNumber))
        (Variables|Default|SetbIsAttacking false))
      (:then_1
        (Default|AddScore (Variables|Default|GetBP%20Player%20REF) (Variables|Default|GetScore%20To%20Add%20To%20Player)))
      (:then_2
        (Utilities|FlowControl|Delay 3.0)
        (Actor|DestroyActor)))))

(fn ConstructionScript)